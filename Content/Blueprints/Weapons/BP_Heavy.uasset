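; Heavy weapon Blueprint that spins its Rotator component when fired.
; Each OnFire adds a fixed boost to RotationForce, and Tick rolls the Rotator by that force scaled by delta time.
; While the force is positive, Tick reduces it by a fixed step per frame, so the spin-down depends on frame rate.
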(event `self.ReceiveTick`
  (params (DeltaSeconds :type "Float (single-precision)"))
  (bind _rotationforce (`self.RotationForce`))
  (`SceneComponent.K2_AddRelativeRotation` (`self.Rotator`) (`KismetMathLibrary.MakeRotator` (* DeltaSeconds _rotationforce)) false false)
  (if (> _rotationforce 0.0)
    (set `self.RotationForce` (- _rotationforce 20.0))))

(event `self.OnFire`
  (set `self.RotationForce` (+ (`self.RotationForce`) 400.0)))

(fn `UserConstructionScript`)